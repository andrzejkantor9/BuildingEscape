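; A swinging door actor that opens and closes in response to the OpenDoor OnOpen and OnClose events.
; It caches its rotation at BeginPlay, and the Door_swing timeline adds an OpenAngle yaw to that rotation, playing forward to open and reversing to close.
; Two DoOnce gates, each reset by the opposite event, stop repeated triggers and play a sound at the door for each direction.
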(event `self.ReceiveBeginPlay`
  (set `self.initial rotation` (`self.K2_GetActorRotation`)))

(event `self.OpenDoor.OnOpen`
  (bind _returnvalue (`self.K2_GetActorLocation`))
  (`|ExecutionSequence`
    (:`then_0`
      (goto _label_3 :!via `Reset`))
    (:`then_1`
      (`/Engine/EditorBlueprintResources/StandardMacros.DoOnce` false :!label _label
        (:`Completed`
          (`GameplayStatics.PlaySoundAtLocation` "/Game/door-lock.door-lock" _returnvalue (struct) 1.0 1.0 0.0 null null null)
          (bind (_direction _open_angle) (`Timeline|door_swing` :!label _label_2)
            (:`Update`
              (`self.K2_SetActorRotation` (`KismetMathLibrary.ComposeRotators` (`KismetMathLibrary.MakeRotator` 0.0 0.0 _open_angle) (`self.initial rotation`))))))))))

(event `self.OpenDoor.OnClose`
  (`|ExecutionSequence`
    (:`then_0`
      (goto _label :!via `Reset`))
    (:`then_1`
      (`/Engine/EditorBlueprintResources/StandardMacros.DoOnce` true :!label _label_3
        (:`Completed`
          (`GameplayStatics.PlaySoundAtLocation` "/Game/door-close.door-close" (`self.K2_GetActorLocation`) (struct) 1.0 1.0 0.0 null null null)
          (goto _label_2 :!via `Reverse`))))))

(fn `UserConstructionScript`)