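; Main door Blueprint that swings open and closed in response to OpenDoorLast's OnOpen and OnClose events.
; Opening passes through a DoOnce, plays the door lock sound at the actor's location and runs the Door_swing timeline, whose yaw angle is combined with the rotation stored at BeginPlay.
; Closing resets the DoOnce and reverses the timeline, allowing the door to open again.
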(event `self.ReceiveBeginPlay`
  (set `self.initial rotation` (`self.K2_GetActorRotation`)))

(event `self.OpenDoorLast.OnOpen`
  (`/Engine/EditorBlueprintResources/StandardMacros.DoOnce` false :!label _label
    (:`Completed`
      (`GameplayStatics.PlaySoundAtLocation` "/Game/door-lock.door-lock" (`self.K2_GetActorLocation`) (struct) 1.0 1.0 0.0 null null null)
      (bind (_direction _open_angle) (`Timeline|door_swing` :!label _label_2)
        (:`Update`
          (`self.K2_SetActorRotation` (`KismetMathLibrary.ComposeRotators` (`KismetMathLibrary.MakeRotator` 0.0 0.0 _open_angle) (`self.initial rotation`))))))))

(event `self.OpenDoorLast.OnClose`
  (`|ExecutionSequence`
    (:`then_0`
      (goto _label :!via `Reset`))
    (:`then_1`
      (goto _label_2 :!via `Reverse`))))

(fn `UserConstructionScript`)